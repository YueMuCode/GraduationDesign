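; Player character Blueprint that shows its network role in an overhead widget and adds a test shortcut for the lobby.
; On BeginPlay it casts the OverheadWidget's user widget to BP_DisplayText and passes itself to ShowPlayerNetRole.
; The T key, marked as a testing convenience, calls BeginAlone on the LobbyGameMode, so it only takes effect where that game mode exists.
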(event EventBeginPlay
  (bind _asbp_display_text (Utilities|Casting|CastToBP_DisplayText (UserInterface|GetUserWidgetObject (Variables|Default|GetOverheadWidget))))
  (Class|OverHeadWidget|ShowPlayerNetRole _asbp_display_text self))

(event Collision|EventActorBeginOverlap
  (params (OtherActor :type Actor%20Object%20Reference)))

(event EventTick
  (params (DeltaSeconds :type Float%20%28single-precision%29)))

(event Input|KeyboardEvents|T
  (params (Key :type Key%20Structure :default "None"))
  ;[1 1 1] 方便测试
  (:Pressed
    (bind _aslobby_game_mode (Utilities|Casting|CastToLobbyGameMode (Game|GetGameMode)))
    (if (Utilities|IsValid _aslobby_game_mode)
      (Class|LobbyGameMode|BeginAlone _aslobby_game_mode))))

(fn ConstructionScript)